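; Leaderboard stand for the darts and pong minigames, showing the top 20 scores and the local player's rank.
; GameNumber sets styling and API endpoint; HTTP GET with a JS-supplied wallet string fills the text renders from JSON.
; Dart scores go out through JS, then the board refetches after a delay.
; A trigger box scales hover text via timeline and lets F toggle between player view and GameCamera, locking input.
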(event `SendDartScoreToDB`
  (params (Score :type Integer) (UserName :type String) (GameNumber :type Integer))
  ;[1 1 1] Send Dart Scores to DB
  (`ABrowserCommActor.Comm_SendStringToJS` (`KismetStringLibrary.Concat_StrStr` (`KismetStringLibrary.Conv_IntToString` Score) "_" UserName) GameNumber)
  ;[1 1 1] Get Leaderboards Data from DB
  (`KismetSystemLibrary.Delay` 2.0)
  (bind _output_get (set `self.LeaderboardRequest` (`VaRestRequestJSON.ConstructRequestExt` "GET" "x_www_form_urlencoded_url") :!label _label))
  (add `VaRestRequestJSON.OnRequestComplete` _output_get (delegate `RequestCompleted`))
  (bind _url (`ABrowserCommActor.GetStringFromJS`))
  (if (`self.isNewGame`)
    (set `self.isNewGame` false)
    (switch `int` (`self.gameNumber`)
      (:`0`
        (set `self.getLeaderboardURL` "https://game-lounge-leaderboards.herokuapp.com/api/leaderboard/darts?amount=20&wallet=" :!label _label_2))
      (:`1`
        (set `self.getLeaderboardURL` "https://game-lounge-leaderboards.herokuapp.com/api/leaderboard/pong?amount=20&wallet=" :!label _label_3)))
    (else
      (switch `int` GameNumber
        (:`1`
          (goto _label_2))
        (:`2`
          (goto _label_3)))))
  (`VaRestRequestJSON.ProcessURL` _output_get (`KismetStringLibrary.Concat_StrStr` (`self.getLeaderboardURL`) _url)))

(event `RequestCompleted`
  (params (Request :type "VaRestRequestJSON Object Reference"))
  (bind _returnvalue (`KismetTextLibrary.Conv_StringToText` ""))
  (bind _playernamesarray (`self.playerNamesArray`))
  (bind _ourposition (`self.OurPosition`))
  (bind _gamenumber (`self.gameNumber`))
  (bind _ourposition_2 (`self.OurPosition`))
  (bind _ourposition_3 (`self.OurPosition`))
  (bind _ourposition_4 (`self.OurPosition`))
  ;[1 1 1] Get Leaderboards Data from DB
  (bind _returnvalue_2 (`VaRestRequestJSON.GetResponseObject` Request))
  (for (_array_element _array_index) (`VaRestJsonObject.GetObjectArrayField` _returnvalue_2 "scores")
    (bind _returnvalue_3 (`VaRestJsonObject.GetStringField` (`VaRestJsonObject.GetObjectField` _array_element "player") "name"))
    ;[1 1 1] Set Leaberboard Player Names
    (if (`KismetStringLibrary.EqualEqual_StrStr` _returnvalue_3)
      (`KismetArrayLibrary.Array_Set` _playernamesarray _array_index "-MISSING-<br>")
      (else
        (`KismetArrayLibrary.Array_Set` _playernamesarray _array_index (`KismetStringLibrary.Concat_StrStr` _returnvalue_3 "<br>"))))
    (`KismetArrayLibrary.Array_Set` (`self.playerScoresArray`) _array_index (`VaRestJsonObject.GetNumberField` _array_element "value")))
  (set `self.playerNamesString` "")
  (for _array_element_2 _playernamesarray
    (bind _output_get (set `self.playerNamesString` (`KismetStringLibrary.Concat_StrStr` (`self.playerNamesString`) _array_element_2))))
  (`TextRenderComponent.K2_SetText` (`self.PlayerNames`) (`KismetTextLibrary.Conv_StringToText` _output_get))
  ;[1 1 1] Set Leaberboards Player Scores
  (set `self.playerScoresString` "")
  (for _array_element_3 (`self.playerScoresArray`)
    (bind _output_get_2 (set `self.playerScoresString` (`KismetStringLibrary.Concat_StrStr` (`self.playerScoresString`) (`KismetStringLibrary.LeftChop` (`KismetStringLibrary.Conv_DoubleToString` _array_element_3) 2) "<br>"))))
  (`TextRenderComponent.K2_SetText` (`self.Scores`) (`KismetTextLibrary.Conv_StringToText` _output_get_2))
  ;[1 1 1] Set Our Name and Score
  (if (`KismetStringLibrary.EqualEqual_StrStr` (stale `SendDartScoreToDB` _url))
    (`TextRenderComponent.K2_SetText` (`self.OurName`) _returnvalue)
    (`TextRenderComponent.K2_SetText` (`self.OurScore`) _returnvalue)
    (`TextRenderComponent.K2_SetText` (`self.OurPosition`) _returnvalue)
    (`TextRenderComponent.K2_SetText` (`self.MyScoreText`) _returnvalue)
    (else
      (bind _returnvalue_4 (`VaRestJsonObject.GetObjectField` _returnvalue_2 "myScore"))
      (`TextRenderComponent.K2_SetText` (`self.OurName`) (`KismetTextLibrary.Conv_StringToText` (`VaRestJsonObject.GetStringField` (`VaRestJsonObject.GetObjectField` _returnvalue_4 "player") "name")))
      (`TextRenderComponent.K2_SetText` (`self.OurScore`) (`KismetTextLibrary.Conv_DoubleToText` (`VaRestJsonObject.GetNumberField` _returnvalue_4 "value") "HalfToEven"))
      (bind _returnvalue_5 (`KismetTextLibrary.Conv_DoubleToText` (+ (`VaRestJsonObject.GetNumberField` _returnvalue_4 "position") 1.0) "HalfToEven"))
      (`TextRenderComponent.K2_SetText` (`self.OurPosition`) _returnvalue_5)
      (switch `int` (`KismetStringLibrary.Len` (`KismetTextLibrary.Conv_TextToString` _returnvalue_5))
        (:`1`
          (switch `int` _gamenumber
            (:`0`
              (`TextRenderComponent.SetWorldSize` _ourposition 40.0))
            (:`1`
              (`TextRenderComponent.SetWorldSize` _ourposition 20.0))))
        (:`2`
          (switch `int` _gamenumber
            (:`0`
              (`TextRenderComponent.SetWorldSize` _ourposition_4 40.0))
            (:`1`
              (`TextRenderComponent.SetWorldSize` _ourposition_4 20.0))))
        (:`3`
          (switch `int` _gamenumber
            (:`0`
              (`TextRenderComponent.SetWorldSize` _ourposition_3 30.0))
            (:`1`
              (`TextRenderComponent.SetWorldSize` _ourposition_3 15.0))))
        (:`4`
          (switch `int` _gamenumber
            (:`0`
              (`TextRenderComponent.SetWorldSize` _ourposition_2 25.0))
            (:`1`
              (`TextRenderComponent.SetWorldSize` _ourposition_2 12.0))))))))

(event `self.Box.OnComponentBeginOverlap`
  (params (OverlappedComponent :type "PrimitiveComponent Object Reference") (OtherActor :type "Actor Object Reference") (OtherComp :type "PrimitiveComponent Object Reference") (OtherBodyIndex :type Integer) (bFromSweep :type Boolean) (SweepResult :type "HitResult Structure (by ref)"))
  (bind _asfirst_person_character (cast `/Game/Blueprints/Character/FirstPersonCharacter` OtherActor))
  (if (`Pawn.IsLocallyControlled` _asfirst_person_character)
    (set `self.canStartPlaying` true)
    (`self.ShowText`)))

(event `self.Box.OnComponentEndOverlap`
  (params (OverlappedComponent :type "PrimitiveComponent Object Reference") (OtherActor :type "Actor Object Reference") (OtherComp :type "PrimitiveComponent Object Reference") (OtherBodyIndex :type Integer))
  (bind _asfirst_person_character (cast `/Game/Blueprints/Character/FirstPersonCharacter` OtherActor))
  (if (`Pawn.IsLocallyControlled` _asfirst_person_character)
    (set `self.canStartPlaying` false)
    (`self.HideText`)))

(event `ShowTextEvent`
  (bind _hoveringtext (`self.hoveringText`))
  (bind (_direction _size) (`Timeline|Timeline_0` :!label _label_4)
    (:`Update`
      (`self.SetActorScale3D` _hoveringtext (* (`KismetMathLibrary.MakeVector` _size _size _size) (`self.hoveringTextSize`)))
      (if (== _size 0.0)
        (`SceneComponent.SetVisibility` (`/Game/Blueprints/TextRenderer.TextRender` _hoveringtext) false false)))))

(event `HideTextEvent`
  (goto _label_4 :!via `Reverse`))

(event `self.ReceiveBeginPlay`
  (bind _hoveringtext (`self.hoveringText`))
  (bind _leaderboardtitle (`self.LeaderboardTitle`))
  (`|ExecutionSequence`
    (:`then_0`
      (`self.EnableInput` (`GameplayStatics.GetPlayerController` 0))
      (`SceneComponent.SetVisibility` (`/Game/Blueprints/TextRenderer.TextRender` _hoveringtext) false false)
      (set `self.hoveringTextSize` (`self.GetActorScale3D` _hoveringtext))
      (switch `int` (`self.gameNumber`)
        (:`0`
          (`TextRenderComponent.K2_SetText` _leaderboardtitle (`KismetTextLibrary.Conv_StringToText` "Darts Top 20 Scores"))
          (`TextRenderComponent.SetFont` _leaderboardtitle "/Game/Blueprints/DartGame/Fonts/eraser_dust_offline.eraser_dust_offline")
          (`TextRenderComponent.SetFont` (`self.PlayerNames`) "/Game/Blueprints/DartGame/Fonts/eraser_dust_offline.eraser_dust_offline")
          (`TextRenderComponent.SetFont` (`self.MyScoreText`) "/Game/Blueprints/DartGame/Fonts/eraser_dust_offline.eraser_dust_offline")
          (`TextRenderComponent.SetFont` (`self.PlayerRanks`) "/Game/Blueprints/DartGame/Fonts/eraser_dust_offline.eraser_dust_offline")
          (`TextRenderComponent.SetFont` (`self.OurScore`) "/Game/Blueprints/DartGame/Fonts/eraser_dust_offline.eraser_dust_offline")
          (`TextRenderComponent.SetFont` (`self.OurName`) "/Game/Blueprints/DartGame/Fonts/eraser_dust_offline.eraser_dust_offline")
          (`TextRenderComponent.SetFont` (`self.Scores`) "/Game/Blueprints/DartGame/Fonts/eraser_dust_offline.eraser_dust_offline")
          (`TextRenderComponent.SetFont` (`self.OurPosition`) "/Game/Blueprints/DartGame/Fonts/eraser_dust_offline.eraser_dust_offline")
          (`TextRenderComponent.SetWorldSize` _leaderboardtitle 35.0)
          (`TextRenderComponent.SetWorldSize` (`self.PlayerNames`) 40.0)
          (`TextRenderComponent.SetWorldSize` (`self.MyScoreText`) 40.0)
          (`TextRenderComponent.SetWorldSize` (`self.PlayerRanks`) 40.0)
          (`TextRenderComponent.SetWorldSize` (`self.OurScore`) 40.0)
          (`TextRenderComponent.SetWorldSize` (`self.OurName`) 40.0)
          (`TextRenderComponent.SetWorldSize` (`self.Scores`) 40.0)
          (`TextRenderComponent.SetWorldSize` (`self.OurPosition`) 40.0)
          (`TextRenderComponent.SetVertSpacingAdjust` (`self.PlayerRanks`) -3.894737)
          (`TextRenderComponent.SetVertSpacingAdjust` (`self.PlayerNames`) -3.894737)
          (`TextRenderComponent.SetVertSpacingAdjust` (`self.Scores`) -3.894737))
        (:`1`
          (`TextRenderComponent.K2_SetText` _leaderboardtitle (`KismetTextLibrary.Conv_StringToText` "Pong Top 20 Scores"))
          (`TextRenderComponent.SetFont` _leaderboardtitle "/Game/Fonts/ARCADE_N_OFFLINE.ARCADE_N_OFFLINE")
          (`TextRenderComponent.SetFont` (`self.Scores`) "/Game/Fonts/ARCADE_N_OFFLINE.ARCADE_N_OFFLINE")
          (`TextRenderComponent.SetFont` (`self.OurName`) "/Game/Fonts/ARCADE_N_OFFLINE.ARCADE_N_OFFLINE")
          (`TextRenderComponent.SetFont` (`self.OurScore`) "/Game/Fonts/ARCADE_N_OFFLINE.ARCADE_N_OFFLINE")
          (`TextRenderComponent.SetFont` (`self.PlayerRanks`) "/Game/Fonts/ARCADE_N_OFFLINE.ARCADE_N_OFFLINE")
          (`TextRenderComponent.SetFont` (`self.MyScoreText`) "/Game/Fonts/ARCADE_N_OFFLINE.ARCADE_N_OFFLINE")
          (`TextRenderComponent.SetFont` (`self.PlayerNames`) "/Game/Fonts/ARCADE_N_OFFLINE.ARCADE_N_OFFLINE")
          (`TextRenderComponent.SetFont` (`self.OurPosition`) "/Game/Fonts/ARCADE_N_OFFLINE.ARCADE_N_OFFLINE")
          (`SceneComponent.K2_SetRelativeLocation` _leaderboardtitle (1.022959 -0.238808 21.559938) false false)
          (`TextRenderComponent.SetWorldSize` _leaderboardtitle 15.0)
          (`TextRenderComponent.SetWorldSize` (`self.PlayerNames`) 20.0)
          (`TextRenderComponent.SetWorldSize` (`self.MyScoreText`) 20.0)
          (`TextRenderComponent.SetWorldSize` (`self.PlayerRanks`) 20.0)
          (`TextRenderComponent.SetWorldSize` (`self.OurScore`) 20.0)
          (`TextRenderComponent.SetWorldSize` (`self.OurName`) 20.0)
          (`TextRenderComponent.SetWorldSize` (`self.Scores`) 20.0)
          (`TextRenderComponent.SetWorldSize` (`self.OurPosition`) 20.0)
          (`TextRenderComponent.SetVertSpacingAdjust` (`self.PlayerRanks`) 11.912657)
          (`TextRenderComponent.SetVertSpacingAdjust` (`self.PlayerNames`) 11.912657)
          (`TextRenderComponent.SetVertSpacingAdjust` (`self.Scores`) 11.912657)
          (`SceneComponent.K2_SetRelativeLocation` (`self.MyScoreText`) (1.022959 0.531415 -18.787868) false false))))
    (:`then_1`
      (goto _label))))

(event `Key|F` :consume false
  (params (Key :type "Key Structure"))
  (bind _returnvalue (`GameplayStatics.GetPlayerController` 0))
  (bind _gamecamera (`self.gameCamera`))
  (:`Pressed`
    (if (`self.canStartPlaying`)
      (if (`KismetStringLibrary.EqualEqual_StrStr` (`KismetSystemLibrary.GetObjectName` _gamecamera) (`KismetSystemLibrary.GetObjectName` (`Controller.GetViewTarget` _returnvalue)))
        (`Controller.SetIgnoreMoveInput` _returnvalue false)
        (`Controller.SetIgnoreLookInput` _returnvalue false)
        (`PlayerController.SetViewTargetWithBlend` _returnvalue (`GameplayStatics.GetPlayerCharacter` 0) 0.5 "VTBlend_EaseIn" 0.5 true)
        (`SceneComponent.SetVisibility` (`/Game/Blueprints/TextRenderer.TextRender` (`self.hoveringText`)) true false)
        (else
          (`Controller.SetIgnoreMoveInput` _returnvalue true)
          (`Controller.SetIgnoreLookInput` _returnvalue true)
          (`PlayerController.SetViewTargetWithBlend` _returnvalue _gamecamera 0.5 "VTBlend_EaseIn" 0.5 true)
          (set `self.canStartPlaying` false)
          (`SceneComponent.SetVisibility` (`/Game/Blueprints/TextRenderer.TextRender` (`self.hoveringText`)) false false)
          (`KismetSystemLibrary.Delay` 0.5)
          (set `self.canStartPlaying` true))))))

(fn `HideText`
  (`self.HideTextEvent`))

(fn `ShowText`
  (`SceneComponent.SetVisibility` (`/Game/Blueprints/TextRenderer.TextRender` (`self.hoveringText`)) true false)
  (`self.ShowTextEvent`))

(fn `UserConstructionScript`)