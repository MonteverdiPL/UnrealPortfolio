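; DartBoard_BP is a dartboard actor for a dart game that spins and can be stopped by player input.
; A timeline spins CenterPoint with a rotation lerp from BeginPlay, replaying itself on finish to loop.
; ActionButton flip-flops between Rotate, which restarts the spin, and StopRotate.
; StopRotate halts the spin, then a second timeline lerps Axis from its current relative location toward CenterPoint's.
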(event `self.ReceiveBeginPlay`
  (`self.Rotate`))

(event `Rotate`
  (`KismetSystemLibrary.PrintString` "StartRotating")
  (bind (_direction _alpharotation) (`Timeline|RotatingMovement` :!via `PlayFromStart` :!label _label)
    (:`Update`
      (`SceneComponent.K2_SetRelativeRotation` (`self.CenterPoint`) (`KismetMathLibrary.RLerp` (struct :`Roll` -90.0) (struct :`Yaw` 360.0 :`Roll` -90.0) _alpharotation) false false))
    (:`Finished`
      (`self.Rotate`))))

(event `StopRotate`
  (`KismetSystemLibrary.PrintString` "StopRotating")
  (`|ExecutionSequence`
    (:`then_0`
      (goto _label :!via `Stop`))
    (:`then_1`
      (set `self.Relative Location` (`SceneComponent.RelativeLocation` (`self.Axis`)))
      (bind (_direction _newtrack_0) (`Timeline|MovementForwardbacward` :!via `PlayFromStart`)
        (:`Update`
          (`SceneComponent.K2_SetRelativeLocation` (`self.Axis`) (`KismetMathLibrary.VLerp` (`self.Relative Location`) (`SceneComponent.RelativeLocation` (`self.CenterPoint`)) _newtrack_0) false false))))))

(event `InputAction|ActionButton`
  (params (Key :type "Key Structure"))
  (:`Pressed`
    (`/Engine/EditorBlueprintResources/StandardMacros.FlipFlop`
      (:`A`
        (`self.Rotate`))
      (:`B`
        (`self.StopRotate`)))))

(fn `UserConstructionScript`)