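; DartAim_Bp is the moving aim actor for the dart minigame, sweeping back and forth between two supplied points.
; StartMovement chains two timelines that lerp the actor's location out and back, then calls itself to loop until StopMovment stops both.
; Timeline play rate derives from the dart game controller's difficulty level and second aim speed.
; An unconnected construction-script fragment building control points from the controller's targeting points never runs.
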(event `StartMovement`
  (params (StartPoint :type "Vector Structure") (EndPoint :type "Vector Structure"))
  (bind _dartgamecontroler (`self.DartGameControler`))
  (`TimelineComponent.SetPlayRate` (`self.Timeline_0`) (`KismetMathLibrary.Abs` (/ (`/Game/Blueprints/DartGame/DartGameControler_Bp.DifficultyLevel` _dartgamecontroler) (`KismetMathLibrary.Conv_IntToDouble` (`/Game/Blueprints/DartGame/DartGameControler_Bp.SecondAimSpeed` _dartgamecontroler)))))
  (`TimelineComponent.SetPlayRate` (`self.Timeline_1`) (`KismetMathLibrary.Abs` (/ (`/Game/Blueprints/DartGame/DartGameControler_Bp.DifficultyLevel` _dartgamecontroler) (`KismetMathLibrary.Conv_IntToDouble` (`/Game/Blueprints/DartGame/DartGameControler_Bp.SecondAimSpeed` _dartgamecontroler)))))
  (bind (_direction _newtrack_0) (`Timeline|Timeline_0` :!via `PlayFromStart` :!label _label)
    (:`Update`
      (`self.K2_SetActorLocation` (`KismetMathLibrary.VLerp` StartPoint EndPoint _newtrack_0)))
    (:`Finished`
      (bind (_direction_2 _newtrack_0_2) (`Timeline|Timeline_1` :!via `PlayFromStart` :!label _label_2)
        (:`Update`
          (`self.K2_SetActorLocation` (`KismetMathLibrary.VLerp` EndPoint StartPoint _newtrack_0_2)))
        (:`Finished`
          (`self.StartMovement` StartPoint EndPoint))))))

(event `StopMovment`
  (`|ExecutionSequence`
    (:`then_0`
      (goto _label :!via `Stop`))
    (:`then_1`
      (goto _label_2 :!via `Stop`))))

(fn `UserConstructionScript`)