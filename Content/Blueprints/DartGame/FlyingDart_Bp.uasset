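; FlyingDart_Bp is a short-lived dart actor for the dart game that fades out and removes itself after spawning.
; On BeginPlay it waits briefly, creates a dynamic instance of M_Master_Alpha on DartMesh, and drives its Alpha parameter with the SetAlpha timeline.
; The actor destroys itself when the timeline finishes.
; An unconnected chain that would enable mesh physics before destroying the actor never runs.
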(event `self.ReceiveBeginPlay`
  (`KismetSystemLibrary.Delay` 1.0)
  (bind _returnvalue (`PrimitiveComponent.CreateDynamicMaterialInstance` (`self.DartMesh`) 0 "/Game/Blueprints/DartGame/M_Master_Alpha.M_Master_Alpha" "None"))
  (bind (_direction _newtrack_0) (`Timeline|set alpha` :!via `PlayFromStart`)
    (:`Update`
      (`MaterialInstanceDynamic.SetScalarParameterValue` _returnvalue "Alpha" _newtrack_0))
    (:`Finished`
      (`self.K2_DestroyActor`))))

(fn `UserConstructionScript`)