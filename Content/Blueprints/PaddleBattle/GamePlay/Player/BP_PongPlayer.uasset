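; BP_PongPlayer spawns and drives both paddles in the Pong game, placing them at mirrored distances around an anchor.
; Axis input always moves the right paddle, and the left only in Single or Hot Seat modes.
; Tick steers the left paddle proportionally toward the ball's Y as AI; restarts enable Tick only for Classic mode.
; Game state events for restart and next round reset paddle positions and sizes.
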(event `self.ReceiveBeginPlay`
  (`|ExecutionSequence`
    (:`then_0`
      ;[1 1 1] Spawn Left Paddle
      (bind _location (`self.GetInitialLocationForPlayer` 0))
      (bind _returnvalue (`|SpawnActorFromClass` "/Game/Blueprints/PaddleBattle/GamePlay/Player/BP_PongPaddle.BP_PongPaddle_C" (`KismetMathLibrary.MakeTransform` _location) "Undefined" "OverrideRootScale" self null))
      (bind _output_get (set `self.LeftPaddle` _returnvalue))
      (`PrimitiveComponent.SetMaterial` (`/Game/Blueprints/PaddleBattle/GamePlay/Player/BP_PongPaddle.PaddleMesh` _output_get) 0 "/Game/Materials/MT_PongWhite.MT_PongWhite")
      (set `/Game/Blueprints/PaddleBattle/GamePlay/Player/BP_PongPaddle.PlayerIndex` 0 _output_get))
    (:`then_1`
      ;[1 1 1] Spawn Right Paddle
      (bind _location_2 (`self.GetInitialLocationForPlayer` 1))
      (bind _returnvalue_2 (`|SpawnActorFromClass` "/Game/Blueprints/PaddleBattle/GamePlay/Player/BP_PongPaddle.BP_PongPaddle_C" (`KismetMathLibrary.MakeTransform` _location_2) "Undefined" "OverrideRootScale" self null))
      (bind _output_get_2 (set `self.RightPaddle` _returnvalue_2))
      (`PrimitiveComponent.SetMaterial` (`/Game/Blueprints/PaddleBattle/GamePlay/Player/BP_PongPaddle.PaddleMesh` _output_get_2) 0 "/Game/Materials/MT_PongWhite.MT_PongWhite")
      (set `/Game/Blueprints/PaddleBattle/GamePlay/Player/BP_PongPaddle.PlayerIndex` 1 _output_get_2))
    (:`then_2`
      ;[1 1 1] Handling game events
      (bind _asbp_pong_game_state (cast `/Game/Blueprints/PaddleBattle/GamePlay/BP_PongGameState` (`GameplayStatics.GetGameState`)))
      (add `/Game/Blueprints/PaddleBattle/GamePlay/BP_PongGameState.OnGameRestarted` _asbp_pong_game_state (delegate `GameRestartEvent`))
      (add `/Game/Blueprints/PaddleBattle/GamePlay/BP_PongGameState.OnNextRound` _asbp_pong_game_state (delegate `NextRoundEvent`)))))

(event `NextRoundEvent`
  ;[1 1 1] Handling game events
  (`self.OnNextRound`))

(event `GameRestartEvent`
  ;[1 1 1] Handling game events
  (`self.OnGameRestarted`))

(event `self.ReceiveTick`
  (params (DeltaSeconds :type "Float (single-precision)"))
  ;[1 1 1] Move Paddle AI (on Tick)
  (`self.MovePaddleAI`))

(event `InputAxis|LeftPaddleUp` :consume false
  (params (AxisValue :type "Float (single-precision)"))
  (bind _leftpaddle (`self.LeftPaddle`))
  ;[1 1 1] Left Paddle Up
  (`self.SwitchOnPongGameType`
    (:`Single`
      _)
    (:`HotSeat`
      _))
  (`/Engine/EditorBlueprintResources/StandardMacros.IsValid` _leftpaddle
    (:`Is Valid`
      (`/Game/Blueprints/PaddleBattle/GamePlay/Player/BP_PongPaddle.MovePaddleUp` _leftpaddle (`self.MovementSpeed`) AxisValue (`SceneComponent.RelativeLocation` (`self.TopBounds`))))))

(event `InputAxis|RightPaddleUp`
  (params (AxisValue :type "Float (single-precision)"))
  (bind _rightpaddle (`self.RightPaddle`))
  ;[1 1 1] Right Paddle Up
  (`/Engine/EditorBlueprintResources/StandardMacros.IsValid` _rightpaddle
    (:`Is Valid`
      (`/Game/Blueprints/PaddleBattle/GamePlay/Player/BP_PongPaddle.MovePaddleUp` _rightpaddle (`self.MovementSpeed`) AxisValue (`SceneComponent.RelativeLocation` (`self.TopBounds`))))))

(event `InputAxis|LeftPaddleDown` :consume false
  (params (AxisValue :type "Float (single-precision)"))
  (bind _leftpaddle (`self.LeftPaddle`))
  ;[1 1 1] Left Paddle Down
  (`self.SwitchOnPongGameType`
    (:`Single`
      _)
    (:`HotSeat`
      _))
  (`/Engine/EditorBlueprintResources/StandardMacros.IsValid` _leftpaddle
    (:`Is Valid`
      (`/Game/Blueprints/PaddleBattle/GamePlay/Player/BP_PongPaddle.MovePaddleDown` _leftpaddle (`self.MovementSpeed`) AxisValue (`SceneComponent.RelativeLocation` (`self.BottomBounds`))))))

(event `InputAxis|RightPaddleDown`
  (params (AxisValue :type "Float (single-precision)"))
  (bind _rightpaddle (`self.RightPaddle`))
  ;[1 1 1] Right Paddle Down
  (`/Engine/EditorBlueprintResources/StandardMacros.IsValid` _rightpaddle
    (:`Is Valid`
      (`/Game/Blueprints/PaddleBattle/GamePlay/Player/BP_PongPaddle.MovePaddleDown` _rightpaddle (`self.MovementSpeed`) AxisValue (`SceneComponent.RelativeLocation` (`self.BottomBounds`))))))

(fn `CallPaddleHit`
  (params (Paddle :type "/Game/Blueprints/PaddleBattle/GamePlay/Player/BP_PongPaddle Object Reference") (HitCounter :type Integer))
  (`self.PaddleHit` Paddle HitCounter))

(fn `GetInitialLocationForPlayer`
  (params (PlayerIndex :type Integer))
  (returns (Location :type "Vector Structure"))
  (locals (Result :type "Vector Structure"))
  (bind _paddlesdistance (`self.PaddlesDistance`))
  (bind _y (.y (`SceneComponent.K2_GetComponentLocation` (`self.PaddleAnchor`))))
  (bind _z (.z (`SceneComponent.K2_GetComponentLocation` (`self.PaddleAnchor`))))
  (if (== PlayerIndex 0)
    (set `local.Result` (`KismetMathLibrary.MakeVector` (* _paddlesdistance -1.0) _y _z))
    (else
      (set `local.Result` (`KismetMathLibrary.MakeVector` _paddlesdistance _y _z))))
  (return (`local.Result`)))

(fn `MovePaddleAI`
  (bind _leftpaddle (`self.LeftPaddle`))
  (bind (_returnvalue_x _returnvalue_y) (`KismetMathLibrary.BreakVector` (`SceneComponent.K2_GetComponentLocation` (`/Game/Blueprints/PaddleBattle/GamePlay/Objects/Ball/BP_PongBall.BallMesh` (`self.Ball`)))))
  (bind (_returnvalue_x_2 _returnvalue_y_2) (`KismetMathLibrary.BreakVector` (`SceneComponent.K2_GetComponentLocation` (`/Game/Blueprints/PaddleBattle/GamePlay/Player/BP_PongPaddle.PaddleMesh` (`self.LeftPaddle`)))))
  (bind _returnvalue (- _returnvalue_y_2 _returnvalue_y))
  (if (> (`KismetMathLibrary.Abs` _returnvalue) 0.2)
    (`/Engine/EditorBlueprintResources/StandardMacros.IsValid` _leftpaddle
      (:`Is Valid`
        (`/Game/Blueprints/PaddleBattle/GamePlay/Player/BP_PongPaddle.MovePaddle` _leftpaddle (/ (* _returnvalue -1.0) (`self.AIAprroachSpeed`)) (`SceneComponent.RelativeLocation` (`self.TopBounds`)) (`SceneComponent.RelativeLocation` (`self.BottomBounds`)))))))

(fn `OnGameOver`)

(fn `OnGameRestarted`
  (`self.SetDefaultPaddleLocations`)
  ;[1 1 1] In case we play with AI - enable Tick (which processes AI movement)
  (bind _asbp_pong_game_mode (cast `/Game/Blueprints/PaddleBattle/GamePlay/BP_PongGameMode` (`GameplayStatics.GetGameMode`)))
  (`self.SetActorTickEnabled` (`|EnumEquality` (`/Game/Blueprints/PaddleBattle/GamePlay/BP_PongGameMode.PongGameType` _asbp_pong_game_mode) "NewEnumerator1")))

(fn `OnNextRound`
  (`self.SetDefaultPaddleLocations`))

(fn `SetDefaultPaddleLocations`
  (bind _rightpaddle (`self.RightPaddle`))
  (bind _leftpaddle (`self.LeftPaddle`))
  (`|ExecutionSequence`
    (:`then_0`
      (`/Engine/EditorBlueprintResources/StandardMacros.IsValid` _leftpaddle
        (:`Is Valid`
          (bind _location (`self.GetInitialLocationForPlayer` 0))
          (`SceneComponent.K2_SetRelativeLocation` (`/Game/Blueprints/PaddleBattle/GamePlay/Player/BP_PongPaddle.DefaultSceneRoot` _leftpaddle) _location false false)
          (`/Game/Blueprints/PaddleBattle/GamePlay/Player/BP_PongPaddle.ResetPaddleSize` _leftpaddle))))
    (:`then_1`
      (`/Engine/EditorBlueprintResources/StandardMacros.IsValid` _rightpaddle
        (:`Is Valid`
          (bind _location_2 (`self.GetInitialLocationForPlayer` 1))
          (`SceneComponent.K2_SetRelativeLocation` (`/Game/Blueprints/PaddleBattle/GamePlay/Player/BP_PongPaddle.DefaultSceneRoot` _rightpaddle) _location_2 false false)
          (`/Game/Blueprints/PaddleBattle/GamePlay/Player/BP_PongPaddle.ResetPaddleSize` _rightpaddle))))))

(fn `UserConstructionScript`)