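; Game state for Pong that tracks both players' scores, turns and match flow, broadcasting score, round, power-up, restart and game-over events.
; ScorePoint credits player 0 in Single mode, then applies signed points one by one behind a cooldown that blocks multi-hit overlaps.
; Classic and Hot Seat check the game mode's point limit to end the game or signal the next round.
; Restart and game over swap in their UI widgets.
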(event `ScorePointEvent`
  (params (PlayerIndex :type Integer) (CountNextRound :type Boolean) (PointsCount :type Integer :default 1))
  ;[1 1 1] Score Point event
  (if (`self.CanScorePoint`)
    (for _ (range (`KismetMathLibrary.Abs_Int` PointsCount))
      (`self.ScorePointForPlayer` PlayerIndex PointsCount)
      (`self.IncreaseTurnsCounter`)
      ;;[1 1 1] Avoid multi-hit point when multiple overlaps are detected
      (set `self.CanScorePoint` false)
      (`KismetSystemLibrary.K2_SetTimerDelegate` (delegate `PointScoredCoolDown`) (`self.ScorePointCoolDown`))
      (`self.OnPointScored` PlayerIndex)
      (`self.CheckPointsWinConditions` CountNextRound))))

(event `PointScoredCoolDown`
  ;[1 1 1] Score Point event
  ;;[1 1 1] Avoid multi-hit point when multiple overlaps are detected
  (set `self.CanScorePoint` true))

(event `PongGameOverEvent`
  (bind _gameplayui (`self.GamePlayUI`))
  ;[1 1 1] Game Over event
  (`/Engine/EditorBlueprintResources/StandardMacros.IsValid` _gameplayui
    (:`Is Valid`
      (`Widget.RemoveFromParent` _gameplayui)
      (`self.OnGameOver`)
      (bind _returnvalue (`|CreateWidget` "/Game/Blueprints/PaddleBattle/UI/WB_GameOver.WB_GameOver_C" (`GameplayStatics.GetPlayerController` 0)))
      (`UserWidget.AddToViewport` _returnvalue 0)
      (`GameplayStatics.PlaySound2D` "/Game/Sounds/Pickup_Coin7.Pickup_Coin7" 1.0 1.0 0.0 null null))))

(event `RestartPongGameEvent`
  ;[1 1 1] Restart Game event
  (set `self.PlayerLeft_Score` 0)
  (set `self.PlayerRight_Score` 0)
  (set `self.TurnsCounter` 0)
  (set `self.BounceCounter` 0)
  (set `self.CanScorePoint` true)
  (bind _outactors (`GameplayStatics.GetAllActorsOfClass` "/Game/Blueprints/PaddleBattle/GamePlay/Objects/Ball/BP_PongBall.BP_PongBall_C"))
  (bind _returnvalue (`|CreateWidget` "/Game/Blueprints/PaddleBattle/UI/WB_GamePlayUI.WB_GamePlayUI_C" (`GameplayStatics.GetPlayerController` 0) (`|GetArrayItem` _outactors)))
  (bind _output_get (set `self.GamePlayUI` _returnvalue))
  (`UserWidget.AddToViewport` _output_get 0)
  (`self.OnGameRestarted`))

(fn `CheckPointsWinConditions`
  (params (CountNextRound :type Boolean))
  (bind _asbp_pong_game_mode (cast `/Game/Blueprints/PaddleBattle/GamePlay/BP_PongGameMode` (`GameplayStatics.GetGameMode`)))
  (switch `/Game/Blueprints/PaddleBattle/Enums/EPongGameType` (`/Game/Blueprints/PaddleBattle/GamePlay/BP_PongGameMode.PongGameType` _asbp_pong_game_mode)
    (:`NewEnumerator1`
      _)
    (:`NewEnumerator2`
      _))
  (bind _classicmodepointslimit (`/Game/Blueprints/PaddleBattle/GamePlay/BP_PongGameMode.ClassicModePointsLimit` _asbp_pong_game_mode))
  (if (or (>= (`self.PlayerLeft_Score`) _classicmodepointslimit) (>= (`self.PlayerRight_Score`) _classicmodepointslimit))
    (`self.PongGameOverEvent`)
    (elif CountNextRound
      (`self.OnNextRound`)
      (`GameplayStatics.PlaySound2D` "/Game/Sounds/Pickup_Coin6.Pickup_Coin6" 1.0 1.0 0.0 null null))))

(fn `IncreaseTurnsCounter`
  (`/Engine/EditorBlueprintResources/StandardMacros.IncrementInt` (`self.TurnsCounter`)))

(fn `PongGameOver`
  (`self.PongGameOverEvent`))

(fn `PowerUp`
  (params (PowerUp :type "/Game/Blueprints/PaddleBattle/GamePlay/Objects/PowerUp/BP_AbstractPowerUp Object Reference"))
  (`self.OnPowerUp` PowerUp))

(fn `RestartPongGame`
  (`self.RestartPongGameEvent`))

(fn `ScorePoint`
  (params (PlayerIndex :type Integer) (CountNextRound :type Boolean) (PointsCount :type Integer :default 1))
  (locals (FinalPlayerIndex :type Integer))
  (bind _asbp_pong_game_mode (cast `/Game/Blueprints/PaddleBattle/GamePlay/BP_PongGameMode` (`GameplayStatics.GetGameMode`)))
  (switch `/Game/Blueprints/PaddleBattle/Enums/EPongGameType` (`/Game/Blueprints/PaddleBattle/GamePlay/BP_PongGameMode.PongGameType` _asbp_pong_game_mode)
    (:`NewEnumerator0`
      (set `local.FinalPlayerIndex` 0))
    (:`NewEnumerator1`
      (set `local.FinalPlayerIndex` PlayerIndex :!label _label))
    (:`NewEnumerator2`
      (goto _label)))
  (`self.ScorePointEvent` (`local.FinalPlayerIndex`) CountNextRound PointsCount))

(fn `ScorePointForPlayer`
  (params (PlayerIndex :type Integer) (PointsCount :type Integer))
  (bind _returnvalue (`KismetMathLibrary.SignOfInteger` PointsCount))
  (if (== PlayerIndex 0)
    (set `self.PlayerLeft_Score` (`KismetMathLibrary.Clamp` (+ (`self.PlayerLeft_Score`) (* 1 _returnvalue)) 0 10000000))
    (else
      (set `self.PlayerRight_Score` (`KismetMathLibrary.Clamp` (+ (`self.PlayerRight_Score`) (* 1 _returnvalue)) 0 10000000)))))

(fn `StartNewGame`
  (`self.OnGameOver`)
  (bind _asbp_pong_game_mode (cast `/Game/Blueprints/PaddleBattle/GamePlay/BP_PongGameMode` (`GameplayStatics.GetGameMode`)))
  (`/Game/Blueprints/PaddleBattle/GamePlay/BP_PongGameMode.StartNewGame` _asbp_pong_game_mode)
  (`KismetSystemLibrary.PrintString` "game state"))

(fn `UserConstructionScript`)