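; Pong ball actor for the paddle battle game that moves by physics velocity in the Anchor's space and follows game-state restart, round and game-over events.
; Hits on paddles, board walls and breakable collide walls redirect it; paddle bounces add paddle motion and random spread, with periodic speed-ups.
; Overlaps apply power-ups or hit score walls, which award points or, in Single mode, end the game.
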(event `self.ReceiveBeginPlay`
  (`|ExecutionSequence`
    (:`then_0`
      ;[1 1 1] Save Ball's initial location
      (set `self.InitialLocation` (`SceneComponent.RelativeLocation` (`self.BallMesh`))))
    (:`then_1`
      ;[1 1 1] Register events handling
      (bind _asbp_pong_game_state (cast `/Game/Blueprints/PaddleBattle/GamePlay/BP_PongGameState` (`GameplayStatics.GetGameState`)))
      (add `/Game/Blueprints/PaddleBattle/GamePlay/BP_PongGameState.OnGameOver` _asbp_pong_game_state (delegate `GameOverEvent`))
      (add `/Game/Blueprints/PaddleBattle/GamePlay/BP_PongGameState.OnGameRestarted` _asbp_pong_game_state (delegate `GameRestartEvent`))
      (add `/Game/Blueprints/PaddleBattle/GamePlay/BP_PongGameState.OnPointScored` _asbp_pong_game_state (delegate `PointScoredEvent`))
      (add `/Game/Blueprints/PaddleBattle/GamePlay/BP_PongGameState.OnNextRound` _asbp_pong_game_state (delegate `NextRoundEvent`)))
    (:`then_2`
      (`SceneComponent.SetVisibility` (`self.BallMesh`) false true))))

(event `GameOverEvent`
  ;[1 1 1] Register events handling
  (`self.OnGameOver`))

(event `GameRestartEvent`
  ;[1 1 1] Register events handling
  (`self.OnGameRestarted`))

(event `PointScoredEvent`
  (params (PlayerIndex :type Integer))
  ;[1 1 1] Register events handling
  (`self.OnPointScored`))

(event `NextRoundEvent`
  ;[1 1 1] Register events handling
  (`self.OnNextRound`))

(event `self.ReceiveHit`
  (params (MyComp :type "PrimitiveComponent Object Reference") (Other :type "Actor Object Reference") (OtherComp :type "PrimitiveComponent Object Reference") (bSelfMoved :type Boolean) (HitLocation :type "Vector Structure") (HitNormal :type "Vector Structure") (NormalImpulse :type "Vector Structure") (Hit :type "HitResult Structure (by ref)"))
  ;[1 1 1] Paddle/PongBoardWall/CollideWall hit detection
  (if (!= (`self.LastHitObject`) Other)
    (bind _output_get (set `self.LastHitObject` Other))
    (bind _asbp_pong_paddle (cast `/Game/Blueprints/PaddleBattle/GamePlay/Player/BP_PongPaddle` _output_get)
      (:`then`
        (`self.CollideWithPaddle` _asbp_pong_paddle (`KismetMathLibrary.InverseTransformLocation` (`self.GetTransform` _asbp_pong_paddle) HitLocation)))
      (:`CastFailed`
        (cast `/Game/Blueprints/PaddleBattle/GamePlay/Level/BP_PongBoardWall` Other
          (:`then`
            (`self.CollideWithBoardWall`))
          (:`CastFailed`
            (bind _asbp_collide_wall (cast `/Game/Blueprints/PaddleBattle/GamePlay/Objects/CollideWall/BP_CollideWall` Other))
            (`self.CollideWithCollideWall` _asbp_collide_wall (`KismetMathLibrary.InverseTransformLocation` (`self.GetTransform` _asbp_collide_wall) HitLocation))))))
    (`GameplayStatics.PlaySound2D` "/Game/Sounds/Blip_Select.Blip_Select" 1.0 1.0 0.0 null null)))

(event `self.ReceiveActorBeginOverlap`
  (params (OtherActor :type "Actor Object Reference"))
  ;[1 1 1] Ball overlapping with ScoreWall
  (bind _asbp_pong_score_wall (cast `/Game/Blueprints/PaddleBattle/GamePlay/Level/BP_PongScoreWall` OtherActor)
    (:`then`
      (`self.CollideWithScoreWall` (`/Game/Blueprints/PaddleBattle/GamePlay/Level/BP_PongScoreWall.PlayerIndex` _asbp_pong_score_wall)))
    (:`CastFailed`
      (bind _asbp_abstract_power_up (cast `/Game/Blueprints/PaddleBattle/GamePlay/Objects/PowerUp/BP_AbstractPowerUp` OtherActor))
      (`/Game/Blueprints/PaddleBattle/GamePlay/Objects/PowerUp/BP_AbstractPowerUp.ApplyPowerUpEffect` _asbp_abstract_power_up self (`self.LastBouncedPaddle`))
      (if (`/Game/Blueprints/PaddleBattle/GamePlay/Objects/PowerUp/BP_AbstractPowerUp.IsPositive` _asbp_abstract_power_up)
        (`GameplayStatics.PlaySound2D` "/Game/Sounds/Jump5.Jump5" 1.0 1.0 0.0 null null)
        (else
          (`GameplayStatics.PlaySound2D` "/Game/Sounds/sad_powerUp.sad_powerUp" 1.0 1.0 0.0 null null)))
      (bind _asbp_pong_game_state (cast `/Game/Blueprints/PaddleBattle/GamePlay/BP_PongGameState` (`GameplayStatics.GetGameState`)))
      (`/Game/Blueprints/PaddleBattle/GamePlay/BP_PongGameState.PowerUp` _asbp_pong_game_state _asbp_abstract_power_up)
      (`self.K2_DestroyActor` _asbp_abstract_power_up))))

(fn `CollideWallBounce`
  (params (`Collide Wall` :type "/Game/Blueprints/PaddleBattle/GamePlay/Objects/CollideWall/BP_CollideWall Object Reference") (HitLocation :type "Vector Structure"))
  (bind (_currentspeed_x _currentspeed_y _currentspeed_z) (`KismetMathLibrary.BreakVector` (`self.CurrentSpeed`)))
  (bind _output_get (set `self.CurrentSpeed` (`KismetMathLibrary.MakeVector` (* _currentspeed_x -1.0) (* _currentspeed_y 1.0) _currentspeed_z)))
  (bind _outvector (`self.LocalToWorld` _output_get))
  (`PrimitiveComponent.SetPhysicsLinearVelocity` (`self.BallMesh`) _outvector false "None")
  (bind _speed (`self.GetBallSpeed`))
  (`self.BallSpeedUpdated` _speed))

(fn `CollideWithBoardWall`
  (bind (_currentspeed_x _currentspeed_y _currentspeed_z) (`KismetMathLibrary.BreakVector` (`self.CurrentSpeed`)))
  (bind _output_get (set `self.CurrentSpeed` (`KismetMathLibrary.MakeVector` _currentspeed_x (* _currentspeed_y -1.0) _currentspeed_z)))
  (bind _outvector (`self.LocalToWorld` _output_get))
  (`PrimitiveComponent.SetPhysicsLinearVelocity` (`self.BallMesh`) _outvector false "None")
  (bind _speed (`self.GetBallSpeed`))
  (`self.BallSpeedUpdated` _speed))

(fn `CollideWithCollideWall`
  (params (CollideWall :type "/Game/Blueprints/PaddleBattle/GamePlay/Objects/CollideWall/BP_CollideWall Object Reference") (HitLocation :type "Vector Structure"))
  (`self.CollideWallBounce` CollideWall HitLocation)
  (`self.K2_DestroyActor` CollideWall))

(fn `CollideWithPaddle`
  (params (Paddle :type "/Game/Blueprints/PaddleBattle/GamePlay/Player/BP_PongPaddle Object Reference") (HitLocation :type "Vector Structure"))
  (`self.SwitchOnGameType`
    (:`Single`
      ;[1 1 1] Score point everytime a (either) paddle is hit
      (bind _asbp_pong_game_state (cast `/Game/Blueprints/PaddleBattle/GamePlay/BP_PongGameState` (`GameplayStatics.GetGameState`)))
      (`/Game/Blueprints/PaddleBattle/GamePlay/BP_PongGameState.ScorePoint` _asbp_pong_game_state 0 false 1))
    (:`Classic`
      _)
    (:`Hot Seat`
      _))
  (`self.PaddleBallBounce` Paddle HitLocation)
  (`self.IncreaseBallSpeed`)
  (bind _speed (`self.GetBallSpeed`))
  (`self.BallSpeedUpdated` _speed)
  (bind _result (`/Engine/EditorBlueprintResources/StandardMacros.IncrementInt` (`self.PaddleHitCounter`))
    (:`  `
      (`/Game/Blueprints/PaddleBattle/GamePlay/Player/BP_PongPlayer.CallPaddleHit` (`self.PongPlayer`) Paddle _result)
      (set `self.LastBouncedPaddle` Paddle))))

(fn `CollideWithScoreWall`
  (params (PlayerIndex :type Integer))
  (bind _asbp_pong_game_state (cast `/Game/Blueprints/PaddleBattle/GamePlay/BP_PongGameState` (`GameplayStatics.GetGameState`)))
  (`self.SwitchOnGameType`
    (:`Single`
      (`/Game/Blueprints/PaddleBattle/GamePlay/BP_PongGameState.PongGameOverEvent` _asbp_pong_game_state))
    (:`Classic`
      (`/Game/Blueprints/PaddleBattle/GamePlay/BP_PongGameState.ScorePoint` _asbp_pong_game_state PlayerIndex true 1 :!label _label)
      (`self.StopMoving`))
    (:`Hot Seat`
      (goto _label))))

(fn `GetBallSpeed`
  (returns (Speed :type "Float (double-precision)"))
  (return (`KismetMathLibrary.VSize` (/ (`self.CurrentSpeed`) 100.0))))

(fn `IncreaseBallSpeed`
  (bind _currentspeed (`self.CurrentSpeed`))
  (bind _asbp_pong_game_state (cast `/Game/Blueprints/PaddleBattle/GamePlay/BP_PongGameState` (`GameplayStatics.GetGameState`)))
  (bind _asbp_pong_game_mode (cast `/Game/Blueprints/PaddleBattle/GamePlay/BP_PongGameMode` (`GameplayStatics.GetGameMode`)))
  (if (== (mod (`/Game/Blueprints/PaddleBattle/GamePlay/BP_PongGameState.BounceCounter` _asbp_pong_game_state) (`/Game/Blueprints/PaddleBattle/GamePlay/BP_PongGameMode.BallSpeedIncreaseTurns` _asbp_pong_game_mode)) 0)
    (bind _output_get (set `self.CurrentSpeed` (+ _currentspeed (* _currentspeed (`/Game/Blueprints/PaddleBattle/GamePlay/BP_PongGameMode.BallSpeedIncreaseAmount` _asbp_pong_game_mode)))))
    (bind _outvector (`self.LocalToWorld` _output_get))
    (`PrimitiveComponent.SetPhysicsLinearVelocity` (`self.BallMesh`) _outvector false "None")
    (bind _speed (`self.GetBallSpeed`))
    (`self.BallSpeedUpdated` _speed)))

(fn `LocalToWorld`
  (params (Vector :type "Vector Structure"))
  (returns (OutVector :type "Vector Structure"))
  (return (`KismetMathLibrary.InverseTransformDirection` (`SceneComponent.K2_GetComponentToWorld` (`self.Anchor`)) Vector)))

(fn `OnGameOver`
  (`self.StopMoving`)
  (set `self.FaceRight` true))

(fn `OnGameRestarted`
  (bind _ballmesh (`self.BallMesh`))
  (`SceneComponent.K2_SetRelativeLocation` _ballmesh (`self.InitialLocation`) false true)
  (`PrimitiveComponent.SetSimulatePhysics` _ballmesh true)
  (`PrimitiveComponent.SetCollisionEnabled` _ballmesh "QueryAndPhysics")
  (bind _returnvalue (`KismetSystemLibrary.K2_SetTimerDelegate` (`|CreateDelegate` :!event `StartMoving`) 1.0))
  (set `self.StartTimer` _returnvalue)
  (set `self.PaddleHitCounter` 0))

(fn `OnNextRound`
  (`KismetSystemLibrary.K2_SetTimerDelegate` (`|CreateDelegate` :!event `StartMoving`) (`self.WaitTimeBetweenRounds`))
  (set `self.PaddleHitCounter` 0))

(fn `OnPointScored`)

(fn `PaddleBallBounce`
  (params (Paddle :type "/Game/Blueprints/PaddleBattle/GamePlay/Player/BP_PongPaddle Object Reference") (HitLocation :type "Vector Structure"))
  (bind _paddlebouncerandomspread (`self.PaddleBounceRandomSpread`))
  (bind (_currentspeed_x _currentspeed_y _currentspeed_z) (`KismetMathLibrary.BreakVector` (`self.CurrentSpeed`)))
  (bind (_currentspeed_x_2 _currentspeed_y_2) (`KismetMathLibrary.BreakVector` (`self.CurrentSpeed`)))
  (bind _returnvalue (`PrimitiveComponent.GetPhysicsLinearVelocity` (`/Game/Blueprints/PaddleBattle/GamePlay/Player/BP_PongPaddle.BounceBox` Paddle) "None"))
  (bind (_returnvalue_x _returnvalue_y) (`KismetMathLibrary.BreakVector` (* (`KismetMathLibrary.Normal` (`KismetMathLibrary.MakeVector` 0.0 (+ (.y _returnvalue) (* HitLocation_Y -1.0) _currentspeed_y_2))) 200.0)))
  (bind _output_get (set `self.CurrentSpeed` (`KismetMathLibrary.MakeVector` (* _currentspeed_x -1.0) (+ _returnvalue_y (`KismetMathLibrary.RandomFloatInRange` (* _paddlebouncerandomspread -1.0) _paddlebouncerandomspread)) _currentspeed_z)))
  (bind _outvector (`self.LocalToWorld` _output_get))
  (`PrimitiveComponent.SetPhysicsLinearVelocity` (`self.BallMesh`) _outvector false "None")
  (bind _speed (`self.GetBallSpeed`))
  (`self.BallSpeedUpdated` _speed)
  (bind _asbp_pong_game_state (cast `/Game/Blueprints/PaddleBattle/GamePlay/BP_PongGameState` (`GameplayStatics.GetGameState`)))
  (`/Engine/EditorBlueprintResources/StandardMacros.IncrementInt` (`/Game/Blueprints/PaddleBattle/GamePlay/BP_PongGameState.BounceCounter` _asbp_pong_game_state)))

(fn `SlowDown`
  (bind _currentspeed (`self.CurrentSpeed`))
  (bind _asbp_pong_game_mode (cast `/Game/Blueprints/PaddleBattle/GamePlay/BP_PongGameMode` (`GameplayStatics.GetGameMode`)))
  (bind _output_get (set `self.CurrentSpeed` (- _currentspeed (* _currentspeed (`/Game/Blueprints/PaddleBattle/GamePlay/BP_PongGameMode.BallSpeedDecreaseAmount` _asbp_pong_game_mode)))))
  (bind _outvector (`self.LocalToWorld` _output_get))
  (`PrimitiveComponent.SetPhysicsLinearVelocity` (`self.BallMesh`) _outvector false "None")
  (bind _speed (`self.GetBallSpeed`))
  (`self.BallSpeedUpdated` _speed))

(fn `SpeedUp`
  (bind _currentspeed (`self.CurrentSpeed`))
  (bind _asbp_pong_game_mode (cast `/Game/Blueprints/PaddleBattle/GamePlay/BP_PongGameMode` (`GameplayStatics.GetGameMode`)))
  (bind _output_get (set `self.CurrentSpeed` (+ _currentspeed (* _currentspeed (`/Game/Blueprints/PaddleBattle/GamePlay/BP_PongGameMode.BallSpeedIncreaseAmount` _asbp_pong_game_mode)))))
  (bind _outvector (`self.LocalToWorld` _output_get))
  (`PrimitiveComponent.SetPhysicsLinearVelocity` (`self.BallMesh`) _outvector false "None")
  (bind _speed (`self.GetBallSpeed`))
  (`self.BallSpeedUpdated` _speed))

(fn `StartMoving`
  (locals (Velocity :type "Vector Structure"))
  (bind _ballmesh (`self.BallMesh`))
  (set `self.LastBouncedPaddle` null)
  (set `self.LastHitObject` null)
  (`PrimitiveComponent.SetSimulatePhysics` _ballmesh true)
  (`PrimitiveComponent.SetCollisionEnabled` _ballmesh "QueryAndPhysics")
  (`SceneComponent.SetVisibility` _ballmesh true true)
  (set `self.CurrentSpeed` (`KismetMathLibrary.MakeVector` (`KismetMathLibrary.Abs` (`self.InitialVelocity`))))
  (if (not (`self.FaceRight`))
    (bind _output_get (set `self.CurrentSpeed` (* (`self.CurrentSpeed`) -1.0))))
  (bind _outvector (`self.LocalToWorld` _output_get))
  (`PrimitiveComponent.SetPhysicsLinearVelocity` (`self.BallMesh`) _outvector false "None")
  (set `self.FaceRight` (not (`self.FaceRight`)))
  (bind _speed (`self.GetBallSpeed`))
  (`self.BallSpeedUpdated` _speed))

(fn `StopMoving`
  (bind _starttimer (`self.StartTimer`))
  (bind _ballmesh (`self.BallMesh`))
  (`PrimitiveComponent.SetPhysicsLinearVelocity` _ballmesh (0.0 0.0 0.0) false "None")
  (`SceneComponent.SetVisibility` _ballmesh false true)
  (`PrimitiveComponent.SetSimulatePhysics` _ballmesh false)
  (`PrimitiveComponent.SetCollisionEnabled` _ballmesh "NoCollision")
  (`SceneComponent.K2_SetRelativeLocation` _ballmesh (`self.InitialLocation`) false true)
  (if (`KismetSystemLibrary.K2_IsValidTimerHandle` _starttimer)
    (`KismetSystemLibrary.K2_ClearAndInvalidateTimerHandle` _starttimer)))

(fn `UserConstructionScript`)

(fn `WorldToLocal`
  (params (Vector :type "Vector Structure"))
  (returns (OutVector :type "Vector Structure"))
  (return (`KismetMathLibrary.TransformDirection` (`SceneComponent.K2_GetComponentToWorld` (`self.Anchor`)) Vector)))