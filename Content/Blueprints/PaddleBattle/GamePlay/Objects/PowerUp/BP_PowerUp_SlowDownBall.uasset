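; A Paddle Battle power-up that slows the ball down.
; It overrides the parent power-up's effect event to call SlowDown on the passed ball if valid, leaving the slowdown logic to the ball.
; It also supplies its own label, "Ball Slow Down", and a green color through getter functions.
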(event `self.ReceiveBeginPlay`
  (`parent.ReceiveBeginPlay`))

(event `/Game/Blueprints/PaddleBattle/GamePlay/Objects/PowerUp/BPI_PowerUpEffect.ApplyPowerUpEffect`
  (params (Ball :type "/Game/Blueprints/PaddleBattle/GamePlay/Objects/Ball/BP_PongBall Object Reference") (Paddle :type "/Game/Blueprints/PaddleBattle/GamePlay/Player/BP_PongPaddle Object Reference"))
  (`/Engine/EditorBlueprintResources/StandardMacros.IsValid` Ball
    (:`Is Valid`
      (`/Game/Blueprints/PaddleBattle/GamePlay/Objects/Ball/BP_PongBall.SlowDown` Ball))))

(fn `GetPowerUpColor`
  (returns (Color :type "SlateColor Structure"))
  (return (make `SlateColor` (struct :`G` 0.473532 :`B` 0.002125 :`A` 1.0))))

(fn `GetPowerUpText`
  (returns (PowerUpText :type Text))
  (return "Ball Slow Down"))

(fn `UserConstructionScript`
  (`parent.UserConstructionScript`))