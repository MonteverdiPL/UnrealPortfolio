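; NFTChanger is a switchable picture display that shows one material from an array of available pictures on its static mesh.
; The construction script applies the material at the current index to slot 2, falling back to the first entry if that one is invalid.
; NextPicture and PreviousPicture step the index with wrap-around at both ends, then reapply the material to the same slot.
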(fn `NextPicture`
  (bind _actualpictureindex (`self.ActualPictureIndex`))
  (if (== _actualpictureindex (- (`KismetArrayLibrary.Array_Length` (`self.AvailablePictures`)) 1))
    (set `self.ActualPictureIndex` 0)
    (else
      (bind _result (`/Engine/EditorBlueprintResources/StandardMacros.IncrementInt` _actualpictureindex)
        (:`  `
          (set `self.ActualPictureIndex` _result)))))
  (`PrimitiveComponent.SetMaterial` (`self.StaticMesh`) 2 (`|GetArrayItem` (`self.AvailablePictures`) (`self.ActualPictureIndex`))))

(fn `PreviousPicture`
  (bind _actualpictureindex (`self.ActualPictureIndex`))
  (if (== _actualpictureindex 0)
    (set `self.ActualPictureIndex` (- (`KismetArrayLibrary.Array_Length` (`self.AvailablePictures`)) 1))
    (else
      (bind _result (`/Engine/EditorBlueprintResources/StandardMacros.DecrementInt` _actualpictureindex)
        (:`  `
          (set `self.ActualPictureIndex` _result)))))
  (`PrimitiveComponent.SetMaterial` (`self.StaticMesh`) 2 (`|GetArrayItem` (`self.AvailablePictures`) (`self.ActualPictureIndex`))))

(fn `UserConstructionScript`
  (bind _staticmesh (`self.StaticMesh`))
  (bind _output (`|GetArrayItem` (`self.AvailablePictures`) (`self.ActualPictureIndex`)))
  (if (`KismetSystemLibrary.IsValid` _output)
    (`PrimitiveComponent.SetMaterial` _staticmesh 2 _output)
    (else
      (`PrimitiveComponent.SetMaterial` _staticmesh 2 (`|GetArrayItem` (`self.AvailablePictures`))))))