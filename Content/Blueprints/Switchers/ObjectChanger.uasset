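; ObjectChanger is an interactive switcher actor that lets the player swap the item spawned at its location.
; BeginPlay spawns the default item and creates a UI_Change_Assets widget; ChangeItem replaces the item with another available class.
; Pressing E, when allowed, locks movement and look, blends to GameCamera and opens the widget; HideUI restores player control.
; A timeline scales the hovering prompt text, which can rotate to face the player on Tick.
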(event `self.ReceiveBeginPlay`
  (bind _hoveringtext (`self.hoveringText`))
  (`self.EnableInput` (`GameplayStatics.GetPlayerController` 0))
  (bind _returnvalue (`|SpawnActorFromClass` (`|GetArrayItem` (`self.AvailableItems`) (`self.DefaultItem`)) (`self.GetTransform`) "Undefined" "OverrideRootScale" null null))
  (set `self.ActualItem` _returnvalue)
  (`SceneComponent.SetVisibility` (`/Game/Blueprints/TextRenderer.TextRender` _hoveringtext) false false)
  (set `self.hoveringTextSize` (`self.GetActorScale3D` _hoveringtext))
  (bind _returnvalue_2 (`|CreateWidget` "/Game/TG_Pack_Vol1/Blueprints/UserInterface/UI_Change_Assets.UI_Change_Assets_C" (`GameplayStatics.GetPlayerController` 0)))
  (set `self.objectChangerWidget` _returnvalue_2)
  (set `self.actualItemNumber` (`self.DefaultItem`)))

(event `ShowTextEvent`
  (bind _hoveringtext (`self.hoveringText`))
  (bind (_direction _size) (`Timeline|TextSize` :!label _label)
    (:`Update`
      (`self.SetActorScale3D` _hoveringtext (* (`KismetMathLibrary.MakeVector` _size _size _size) (`self.hoveringTextSize`)))
      (if (== _size 0.0)
        (`SceneComponent.SetVisibility` (`/Game/Blueprints/TextRenderer.TextRender` _hoveringtext) false false)))))

(event `HideTextEvent`
  (goto _label :!via `Reverse`))

(event `Key|E` :consume false
  (params (Key :type "Key Structure"))
  (bind _returnvalue (`GameplayStatics.GetPlayerController` 0))
  (bind _objectchangerwidget (`self.objectChangerWidget`))
  (:`Pressed`
    (if (`self.canStartPlaying`)
      (if (not (`self.isUIActive`))
        (`Controller.SetIgnoreMoveInput` _returnvalue true)
        (`Controller.SetIgnoreLookInput` _returnvalue true)
        (`PlayerController.SetViewTargetWithBlend` _returnvalue (`self.gameCamera`) 0.5 "VTBlend_EaseIn" 0.5 true)
        (set `self.isUIActive` true)
        (`SceneComponent.SetVisibility` (`/Game/Blueprints/TextRenderer.TextRender` (`self.hoveringText`)) false false)
        (`KismetSystemLibrary.Delay` 0.5)
        (`UserWidget.AddToViewport` _objectchangerwidget 0)
        (`GameplayStatics.SetViewportMouseCaptureMode` "NoCapture")
        (set `self.canStartPlaying` true)
        (`/Game/TG_Pack_Vol1/Blueprints/UserInterface/UI_Change_Assets.setActualObjectChanger` _objectchangerwidget self)
        (`/Game/TG_Pack_Vol1/Blueprints/UserInterface/UI_Change_Assets.setButtonSelectionOnCreation` _objectchangerwidget (`self.actualItemNumber`))
        (`/Game/TG_Pack_Vol1/Blueprints/UserInterface/UI_Change_Assets.setAvailableItems` _objectchangerwidget (`KismetArrayLibrary.Array_Length` (`self.ItemPictures`)))
        (`/Game/TG_Pack_Vol1/Blueprints/UserInterface/UI_Change_Assets.setItemTitles` _objectchangerwidget (`self.itemTitles`))
        (bind _asfirst_person_character (cast `/Game/Blueprints/Character/FirstPersonCharacter` (`GameplayStatics.GetPlayerCharacter` 0)))
        (set `/Game/Blueprints/Character/FirstPersonCharacter.isUIActive` true _asfirst_person_character)))))

(event `HideUI`
  (bind _returnvalue (`GameplayStatics.GetPlayerController` 0))
  (`Controller.SetIgnoreMoveInput` _returnvalue false)
  (`Controller.SetIgnoreLookInput` _returnvalue false)
  (`PlayerController.SetViewTargetWithBlend` _returnvalue (`GameplayStatics.GetPlayerCharacter` 0) 0.5 "VTBlend_EaseIn" 0.5 true)
  (`SceneComponent.SetVisibility` (`/Game/Blueprints/TextRenderer.TextRender` (`self.hoveringText`)) true false)
  (`Widget.RemoveFromParent` (`self.objectChangerWidget`))
  (set `self.isUIActive` false)
  (bind _asfirst_person_character (cast `/Game/Blueprints/Character/FirstPersonCharacter` (`GameplayStatics.GetPlayerCharacter` 0)))
  (set `/Game/Blueprints/Character/FirstPersonCharacter.isUIActive` false _asfirst_person_character))

(event `self.ReceiveTick`
  (params (DeltaSeconds :type "Float (single-precision)"))
  (bind _hoveringtext (`self.hoveringText`))
  (if (`self.followingText`)
    (`self.K2_SetActorRotation` _hoveringtext (`KismetMathLibrary.FindLookAtRotation` (`self.K2_GetActorLocation` _hoveringtext) (+ (`self.K2_GetActorLocation` (`GameplayStatics.GetPlayerCharacter` 0)) (0.0 0.0 40.0))) false)))

(fn `ChangeItem`
  (params (ItemNumber :type Integer))
  (if (`KismetSystemLibrary.IsValidClass` (`|GetArrayItem` (`self.AvailableItems`) ItemNumber))
    (`self.K2_DestroyActor` (`self.ActualItem`))
    (bind _returnvalue (`|SpawnActorFromClass` (`|GetArrayItem` (`self.AvailableItems`) ItemNumber) (`self.GetTransform`) "Undefined" "OverrideRootScale" null null))
    (set `self.ActualItem` _returnvalue)
    (set `self.actualItemNumber` ItemNumber)))

(fn `HideText`
  (`self.HideTextEvent`))

(fn `ShowText`
  (`SceneComponent.SetVisibility` (`/Game/Blueprints/TextRenderer.TextRender` (`self.hoveringText`)) true false)
  (`self.ShowTextEvent`))

(fn `UserConstructionScript`)