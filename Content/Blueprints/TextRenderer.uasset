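; TextRenderer is a Blueprint that displays a configurable Text value through a TextRender component.
; The construction script sets the text, then repositions the component relative to its parent using offsets derived from half its measured local width and height, so placement follows the text's size.
; The event graph has no active logic.
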(event `self.ReceiveBeginPlay`)

(fn `UserConstructionScript`
  (bind _textrender (`self.TextRender`))
  (`TextRenderComponent.K2_SetText` (`self.TextRender`) (`self.Text`))
  (bind _result (`/Engine/EditorBlueprintResources/StandardMacros.NegateFloat` (/ (.z (`TextRenderComponent.GetTextLocalSize` _textrender)) 2.0))
    (:`  `
      (`SceneComponent.K2_SetRelativeLocation` _textrender (`KismetMathLibrary.MakeVector` 0.0 (/ (.y (`TextRenderComponent.GetTextLocalSize` _textrender)) 2.0) _result) false false))))