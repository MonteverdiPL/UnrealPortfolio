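; BP_Football_Table is a football table prop that offers two color versions.
; The construction script uses the ColorVersion2 flag to select the ColorVer1 or ColorVer2 material set as CurrentColorVersion.
; It applies the first two materials of that set to the static mesh's first two slots.
; The event graph holds only disabled placeholder events, so the asset has no runtime logic of its own.
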(fn `UserConstructionScript`
  (bind _staticmesh (`self.StaticMesh`))
  (bind _currentcolorversion (`self.CurrentColorVersion`))
  (if (`self.Color Version 2`)
    (set `self.CurrentColorVersion` (`self.ColorVer_2`))
    (else
      (set `self.CurrentColorVersion` (`self.ColorVer_1`))))
  (`PrimitiveComponent.SetMaterial` _staticmesh 0 (`|GetArrayItem` _currentcolorversion))
  (`PrimitiveComponent.SetMaterial` _staticmesh 1 (`|GetArrayItem` _currentcolorversion 1)))